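; Blueprint function library for a studio lighting kit, with helpers for DMX-driven light fixtures and color temperature.
; Kelvin lookups, by enum or string, read the KelvinTorgb data table and normalize RGB to 0–1.
; ScaleDMX functions clamp-remap DMX values into float, truncated int, color, or rotation offset from a current value.
; DMX_DimRGB applies color and divided intensity to a point light, mirroring color and raw intensity into mesh custom primitive data.
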(fn `DMX_DimRGB`
  (params (Color :type "LinearColor Structure") (Intensity :type "Float (double-precision)") (IntensityDivision :type "Float (double-precision)") (PointLight :type "PointLightComponent Object Reference") (StaticMesh :type "StaticMeshComponent Object Reference"))
  (`LightComponent.SetLightColor` PointLight Color true)
  (`LightComponent.SetIntensity` PointLight (/ Intensity IntensityDivision))
  (`PrimitiveComponent.SetCustomPrimitiveDataVector3` StaticMesh 0 (`KismetMathLibrary.Conv_LinearColorToVector` Color))
  (`PrimitiveComponent.SetCustomPrimitiveDataFloat` StaticMesh 4 Intensity))

(fn `KelvinStringsToRGBA`
  (params (Kelvin :type String))
  (returns (RGBA :type "LinearColor Structure"))
  (locals (KelvinValues :type "/TechvizSharedAssets/StudioLightingKit/BluePrints/ENU_KelvinValue Enum" :default "NewEnumerator0"))
  (bind _returnvalue (`|GetDataTableRow` "/TechvizSharedAssets/StudioLightingKit/BluePrints/KelvinTorgb.KelvinTorgb" (`KismetStringLibrary.Conv_StringToName` Kelvin))
    (:`then`
      (bind (_kelvin _r _g _b _a) (break `/TechvizSharedAssets/StudioLightingKit/BluePrints/STRU_Kelvin` _returnvalue))
      (return (make `LinearColor` (/ _r 255.0) (/ _g 255.0) (/ _b 255.0) _a)))))

(fn `KelvinToRGBA`
  (params (Kelvin :type "/TechvizSharedAssets/StudioLightingKit/BluePrints/ENU_KelvinValue Enum" :default "NewEnumerator0"))
  (returns (RGBA :type "LinearColor Structure"))
  (locals (KelvinValues :type "/TechvizSharedAssets/StudioLightingKit/BluePrints/ENU_KelvinValue Enum" :default "NewEnumerator0"))
  (bind _returnvalue (`|GetDataTableRow` "/TechvizSharedAssets/StudioLightingKit/BluePrints/KelvinTorgb.KelvinTorgb" (`KismetStringLibrary.Conv_StringToName` (`|GetEnumeratorNameAsString` Kelvin)))
    (:`then`
      (bind (_kelvin _r _g _b _a) (break `/TechvizSharedAssets/StudioLightingKit/BluePrints/STRU_Kelvin` _returnvalue))
      (return (make `LinearColor` (/ _r 255.0) (/ _g 255.0) (/ _b 255.0) _a)))))

(fn `ScaleDMX_Color`
  (params (r :type Integer) (g :type Integer) (b :type Integer) (`In DMX Range` :type "Array of Float (double-precision)") (`Out Scaled Range` :type "Array of Float (double-precision)"))
  (returns (`Scaled Color` :type "LinearColor Structure"))
  (bind _output (`|GetArrayItem` `Out Scaled Range` 1))
  (bind _output_2 (`|GetArrayItem` `Out Scaled Range`))
  (bind _output_3 (`|GetArrayItem` `In DMX Range`))
  (bind _output_4 (`|GetArrayItem` `In DMX Range` 1))
  (return (make `LinearColor` (`KismetMathLibrary.MapRangeClamped` (`KismetMathLibrary.Conv_IntToDouble` r) _output_3 _output_4 _output_2 _output) (`KismetMathLibrary.MapRangeClamped` (`KismetMathLibrary.Conv_IntToDouble` g) _output_3 _output_4 _output_2 _output) (`KismetMathLibrary.MapRangeClamped` (`KismetMathLibrary.Conv_IntToDouble` b) _output_3 _output_4 _output_2 _output) 1.0)))

(fn `ScaleDMX_Float`
  (params (Value :type Integer) (inDmxRange :type "Array of Float (double-precision)") (OutScaledRange :type "Array of Float (double-precision)"))
  (returns (ScaledValue :type "Float (double-precision)"))
  (return (`KismetMathLibrary.MapRangeClamped` (`KismetMathLibrary.Conv_IntToDouble` Value) (`|GetArrayItem` inDmxRange) (`|GetArrayItem` inDmxRange 1) (`|GetArrayItem` OutScaledRange) (`|GetArrayItem` OutScaledRange 1))))

(fn `ScaleDMX_Int`
  (params (Value :type Integer) (inDmxRange :type "Array of Float (double-precision)") (OutScaledRange :type "Array of Float (double-precision)"))
  (returns (ScaledValue :type Integer))
  (return (`KismetMathLibrary.FTrunc` (`KismetMathLibrary.MapRangeClamped` (`KismetMathLibrary.Conv_IntToDouble` Value) (`|GetArrayItem` inDmxRange) (`|GetArrayItem` inDmxRange 1) (`|GetArrayItem` OutScaledRange) (`|GetArrayItem` OutScaledRange 1)))))

(fn `ScaleDMX_Rotation`
  (params (Value :type Integer) (CurrentValue :type "Float (double-precision)") (InDMX_Range :type "Array of Float (double-precision)") (OutRotationRange :type "Array of Float (double-precision)"))
  (returns (ScaledValue :type "Float (double-precision)"))
  (return (+ (`KismetMathLibrary.MapRangeClamped` (`KismetMathLibrary.Conv_IntToDouble` Value) (`|GetArrayItem` InDMX_Range) (`|GetArrayItem` InDMX_Range 1) (`|GetArrayItem` OutRotationRange) (`|GetArrayItem` OutRotationRange 1)) CurrentValue)))