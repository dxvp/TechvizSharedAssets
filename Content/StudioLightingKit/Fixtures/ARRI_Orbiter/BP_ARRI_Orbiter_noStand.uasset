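; ARRI Orbiter studio light fixture without stand, with selectable optics, body tilt, adjustable leaves and optional DMX control.
; OrbiterFunctions runs on construction, on BeginPlay without DMX, or on received DMX dimmer, color temperature and RGB.
; The chosen optic's DT_OrbiterDOP row configures one of three lights (spot, dome or SP) with transform, IES and source size.
; Color and intensity also drive the optic mesh through Custom Primitive Data.
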(event `self.DMX.OnFixturePatchReceived`
  (params (FixturePatch :type "DMXEntityFixturePatch Object Reference") (ValuePerAttribute :type "DMXNormalizedAttributeValueMap Structure (by ref)"))
  (if (`self.DMX Active`)
    (bind _outattributesmap (`|GetDMXAttributeValues` FixturePatch))
    (bind (_dimmer _colortemperature _tint _colorcrossfade _red _green _blue) (`self.DMXValues` _outattributesmap))
    (bind _scaledvalue (`/TechvizSharedAssets/StudioLightingKit/BluePrints/BP_FunctionLibrary.ScaleDMX_Float` _dimmer (`self.In Dmx Range`) (`self.Intensity Range`)))
    (`self.Dmx to Kelvin Function` _colortemperature)
    (bind _scaled_color (`/TechvizSharedAssets/StudioLightingKit/BluePrints/BP_FunctionLibrary.ScaleDMX_Color` _red _green _blue (`self.In Dmx Range`) (`self.Color Dmx Range`)))
    (`self.OrbiterFunctions` (`self.TiltBody`) _scaledvalue (`self.DOP List`) (not (`KismetMathLibrary.Conv_IntToBool` _colorcrossfade)) (`KismetStringLibrary.Conv_IntToString` (`self.CurrentColorTemperature`)) _scaled_color (`self.ShadowBias`) (`self.LeafRight`) (`self.LeafLeft`) (`self.LeafTop`) (`self.LeafBottom`))))

(event `self.ReceiveBeginPlay`
  (if (not (`self.DMX Active`))
    (`self.OrbiterFunctions` (`self.TiltBody`) (`self.Intensity`) (`self.DOP List`) (`self.Set Temp`) (`|GetEnumeratorNameAsString` (`self.Kelvin`)) (`self.Color`) (`self.ShadowBias`) (`self.LeafRight`) (`self.LeafLeft`) (`self.LeafTop`) (`self.LeafBottom`))))

(fn `Dmx to Kelvin Function`
  (params (`DMX Value` :type Integer))
  (bind _returnvalue (* `DMX Value` 100))
  (if (< _returnvalue 1000)
    (set `self.CurrentColorTemperature` 1000)
    (else
      (bind _output_get (set `self.CurrentColorTemperature` _returnvalue))
      (if (> _output_get 12000)
        (set `self.CurrentColorTemperature` 12000)
        (else
          (set `self.CurrentColorTemperature` _returnvalue)))))
  (return))

(fn `DMXValues`
  (params (`DMX Att` :type "Map of DMXAttributeName Structure to Integer"))
  (returns (Dimmer :type Integer) (ColorTemperature :type Integer) (Tint :type Integer) (ColorCrossFade :type Integer) (Red :type Integer) (Green :type Integer) (Blue :type Integer) (`Dummy 1` :type Integer) (`Dummy 2` :type Integer) (`Dummy 3` :type Integer) (White :type Integer) (CTB :type Integer) (WPTint :type Integer) (Fans :type Integer) (Favorite :type Integer) (Shutter :type Integer) (`Dummy 4` :type Integer))
  (return (`BlueprintMapLibrary.Map_Find` `DMX Att` (struct :`Name` "Dimmer")) (`BlueprintMapLibrary.Map_Find` `DMX Att`) (`BlueprintMapLibrary.Map_Find` `DMX Att` (struct :`Name` "Tint")) (`BlueprintMapLibrary.Map_Find` `DMX Att` (struct :`Name` "CrossFadetoColor")) (`BlueprintMapLibrary.Map_Find` `DMX Att` (struct :`Name` "Red")) (`BlueprintMapLibrary.Map_Find` `DMX Att` (struct :`Name` "Green")) (`BlueprintMapLibrary.Map_Find` `DMX Att` (struct :`Name` "Blue")) 0 0 0 (`BlueprintMapLibrary.Map_Find` `DMX Att` (struct :`Name` "White")) 0 0 (`BlueprintMapLibrary.Map_Find` `DMX Att` (struct :`Name` "Velocity")) (`BlueprintMapLibrary.Map_Find` `DMX Att` (struct :`Name` "Effects")) (`BlueprintMapLibrary.Map_Find` `DMX Att` (struct :`Name` "Shutter")) (`BlueprintMapLibrary.Map_Find` `DMX Att` (struct :`Name` "Dummy 4"))))

(fn `OrbiterFunctions`
  (params (`Tilt Body` :type "Float (double-precision)") (Intensity :type "Float (double-precision)") (`DOP List` :type "/TechvizSharedAssets/StudioLightingKit/BluePrints/ENU_Orbiter_DoP_List Enum" :default "NewEnumerator0") (SetTemp :type Boolean) (Kelvin :type String) (Color :type "LinearColor Structure") (ShadowBias :type "Float (double-precision)") (LeafRight :type "Float (double-precision)") (LeafLeft :type "Float (double-precision)") (LeafTop :type "Float (double-precision)") (LeafBottom :type "Float (double-precision)"))
  (bind (_returnvalue _index) (`self.DOP_List_To_Names` `DOP List`))
  (bind _splight (`self.SPLight`))
  (bind (_dop_datalist_dop_mesh _dop_datalist_mesh_transform _dop_datalist_light_transform _dop_datalist_light_width _dop_datalist_light_height _dop_datalist_source_radius _dop_datalist_ies_texture) (break `/TechvizSharedAssets/StudioLightingKit/BluePrints/STRU_OrbiterDOP` (`self.DOP_DataList`)))
  (bind _lighttype (`self.LightType`))
  (bind _output (`|GetArrayItem` (`self.DOP_Mesh_Array`) _index))
  (`|ExecutionSequence`
    (:`then_0`
      (bind _returnvalue_2 (`|GetDataTableRow` "/TechvizSharedAssets/StudioLightingKit/BluePrints/DT_OrbiterDOP.DT_OrbiterDOP" _returnvalue)
        (:`then`
          (set `self.DOP_Index` _index)
          (set `self.DOP_DataList` _returnvalue_2)
          (`self.SetDOPArray`)
          (`/Engine/EditorBlueprintResources/StandardMacros.IsValid` _output
            (:`Is Valid`
              (if SetTemp
                (bind _rgba (`/TechvizSharedAssets/StudioLightingKit/BluePrints/BP_FunctionLibrary.KelvinStringsToRGBA` Kelvin))
                (set `self.CurrentColor` _rgba)
                (else
                  (set `self.CurrentColor` Color)))
              (`SceneComponent.SetHiddenInGame` _output false false)
              (`SceneComponent.SetVisibility` _output true false)
              (`PrimitiveComponent.SetCustomPrimitiveDataVector3` _output 0 (`KismetMathLibrary.Conv_LinearColorToVector` (`self.CurrentColor`)))
              (`PrimitiveComponent.SetCustomPrimitiveDataFloat` _output 4 (/ Intensity 100.0))
              (switch `int` (`self.DOP_Index`)
                (:`0`
                  (set `self.LightType` (`self.SpotLight`) :!label _label)
                  (`self.SpotLightActive`
                    (:`OUT`
                      _)))
                (:`1`
                  (goto _label))
                (:`2`
                  (goto _label))
                (:`3`
                  (set `self.LightType` (`self.DomeLight`) :!label _label_2)
                  (`self.DomeLightActive`))
                (:`4`
                  (goto _label_2))
                (:`5`
                  (goto _label_2))
                (:`6`
                  (set `self.LightType` (`self.SPLight`) :!label _label_3)
                  (`self.SP_LightActive`))
                (:`7`
                  (goto _label_3))
                (:`8`
                  (goto _label_3)))
              (`SceneComponent.K2_SetRelativeTransform` (`self.LightType`) _dop_datalist_light_transform false false)
              (`PointLightComponent.SetSourceRadius` (`self.DomeLight`) _dop_datalist_source_radius)
              (`LightComponent.SetIESTexture` _lighttype _dop_datalist_ies_texture)
              (`LightComponent.SetIntensity` _lighttype Intensity)
              (`LightComponent.SetLightColor` _lighttype (`self.CurrentColor`) true)
              (`RectLightComponent.SetSourceWidth` _splight _dop_datalist_light_width)
              (`RectLightComponent.SetSourceHeight` _splight _dop_datalist_light_height)
              (`LightComponent.SetShadowBias` _lighttype ShadowBias)
              (`LightComponent.SetShadowBias` _lighttype ShadowBias)
              (`SceneComponent.K2_SetRelativeRotation` (`self.ARRI_Leafs_RightLeaf`) (`KismetMathLibrary.MakeRotator` 0.0 0.0 LeafRight) false false)
              (`SceneComponent.K2_SetRelativeRotation` (`self.ARRI_Leafs_LeftLeaf`) (`KismetMathLibrary.MakeRotator` 0.0 0.0 LeafLeft) false false)
              (`SceneComponent.K2_SetRelativeRotation` (`self.ARRI_Leafs_TopLeaf`) (`KismetMathLibrary.MakeRotator` LeafTop) false false)
              (`SceneComponent.K2_SetRelativeRotation` (`self.ARRI_Leafs_BTMLeaf`) (`KismetMathLibrary.MakeRotator` LeafBottom) false false))))))
    (:`then_1`
      (`SceneComponent.K2_SetRelativeRotation` (`self.Orbiter_body`) (`KismetMathLibrary.MakeRotator` `Tilt Body` 180.0) false false))))

(fn `SetDOPArray`
  (bind _orbiter_body (`self.Orbiter_body`))
  (set `self.DOP_Mesh_Array` (`|MakeArray` _orbiter_body _orbiter_body _orbiter_body (`self.DoP_Dome_L`) (`self.DoP_Dome_M`) (`self.DoP_Dome_S`) (`self.DoP_Octa4_SnapBag`) (`self.DoP_SnapBag_M`) (`self.DoP_SnapBag_S`))))

(fn `UserConstructionScript`
  (`self.OrbiterFunctions` (`self.TiltBody`) (`self.Intensity`) (`self.DOP List`) (`self.Set Temp`) (`|GetEnumeratorNameAsString` (`self.Kelvin`)) (`self.Color`) (`self.ShadowBias`) (`self.LeafRight`) (`self.LeafLeft`) (`self.LeafTop`) (`self.LeafBottom`)))