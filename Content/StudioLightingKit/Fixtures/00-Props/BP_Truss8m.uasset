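; BP_Truss8m is a studio lighting prop: a truss on two stands with adjustable height.
; A Height value sets the relative Z of the left and right stand arms, and places the truss mesh at a fixed offset above that value.
; The same positioning runs in the Construction Script and again on BeginPlay.
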(event `self.ReceiveBeginPlay`
  (bind _height (`self.Height`))
  (`SceneComponent.K2_SetRelativeLocation` (`self.SM_StandArmL`) (`KismetMathLibrary.MakeVector` 0.0 0.0 _height) false false)
  (`SceneComponent.K2_SetRelativeLocation` (`self.SM_StandArmR`) (`KismetMathLibrary.MakeVector` 0.0 0.0 _height) false false)
  (`SceneComponent.K2_SetRelativeLocation` (`self.SM_truss_4m`) (`KismetMathLibrary.MakeVector` 0.0 0.0 (+ _height 303.0)) false false))

(fn `UserConstructionScript`
  (bind _height (`self.Height`))
  (`SceneComponent.K2_SetRelativeLocation` (`self.SM_StandArmL`) (`KismetMathLibrary.MakeVector` 0.0 0.0 _height) false false)
  (`SceneComponent.K2_SetRelativeLocation` (`self.SM_StandArmR`) (`KismetMathLibrary.MakeVector` 0.0 0.0 _height) false false)
  (`SceneComponent.K2_SetRelativeLocation` (`self.SM_truss_4m`) (`KismetMathLibrary.MakeVector` 0.0 0.0 (+ _height 303.0)) false false))