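; ARRI M90 studio light fixture Blueprint with editable tilt, barn doors, hanger, lens, color and intensity.
; M90Functions applies everything to meshes, spot and point lights, picking an IES texture per lens and driving lens glow through custom primitive data.
; Construction script, BeginPlay and optional Tick use manual properties; the latter two only without DMX.
; With DMX active, received patch values set dimmer, clamped Kelvin or RGB color, selected by the crossfade channel.
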(event `self.DMX.OnFixturePatchReceived`
  (params (FixturePatch :type "DMXEntityFixturePatch Object Reference") (ValuePerAttribute :type "DMXNormalizedAttributeValueMap Structure (by ref)"))
  (if (`self.DMX Active`)
    (bind _outattributesmap (`|GetDMXAttributeValues` FixturePatch))
    (bind (_dimmer _colortemperature _tint _colorcrossfade _red _green _blue) (`self.DMXValues` _outattributesmap))
    (bind _scaledvalue (`/TechvizSharedAssets/StudioLightingKit/BluePrints/BP_FunctionLibrary.ScaleDMX_Float` _dimmer (`self.In Dmx Range`) (`self.Intensity Range`)))
    (`self.DmxToKelvinFunction` _colortemperature)
    (bind _scaled_color (`/TechvizSharedAssets/StudioLightingKit/BluePrints/BP_FunctionLibrary.ScaleDMX_Color` _red _green _blue (`self.In Dmx Range`) (`self.Color Dmx Range`)))
    (`self.M90Functions` (`self.TiltBody`) (not (`KismetMathLibrary.Conv_IntToBool` _colorcrossfade)) _scaled_color _scaledvalue (`KismetStringLibrary.Conv_IntToString` (`self.CurrentColorTemperature`)) (`self.ShadowBias`) (`self.LeafRight`) (`self.LeafLeft`) (`self.LeafTop`) (`self.LeafBottom`) (`self.Lens`) (`self.Hide Hang`) (`self.Hide BarnDoor`))))

(event `self.ReceiveBeginPlay`
  (if (not (`self.DMX Active`)) :!label _label
    (`self.M90Functions` (`self.TiltBody`) (`self.Set Temp`) (`self.Color`) (`self.Intensity`) (`|GetEnumeratorNameAsString` (`self.Kelvin`)) (`self.ShadowBias`) (`self.LeafRight`) (`self.LeafLeft`) (`self.LeafTop`) (`self.LeafBottom`) (`self.Lens`) (`self.Hide Hang`) (`self.Hide BarnDoor`))))

(event `self.ReceiveTick`
  (params (DeltaSeconds :type "Float (single-precision)"))
  (if (`self.Event Tick (Play Mode)`)
    (goto _label)))

(fn `DmxToKelvinFunction`
  (params (`DMX Value` :type Integer))
  (bind _returnvalue (* `DMX Value` 100))
  (if (< _returnvalue 1000)
    (set `self.CurrentColorTemperature` 1000)
    (else
      (bind _output_get (set `self.CurrentColorTemperature` _returnvalue))
      (if (> _output_get 12000)
        (set `self.CurrentColorTemperature` 12000)
        (else
          (set `self.CurrentColorTemperature` _returnvalue)))))
  (return))

(fn `DMXValues`
  (params (`DMX Att` :type "Map of DMXAttributeName Structure to Integer"))
  (returns (Dimmer :type Integer) (ColorTemperature :type Integer) (Tint :type Integer) (ColorCrossFade :type Integer) (Red :type Integer) (Green :type Integer) (Blue :type Integer) (White :type Integer) (Fans :type Integer) (ColorPreset :type Integer) (Shutter :type Integer) (Dummy :type Integer))
  (return (`BlueprintMapLibrary.Map_Find` `DMX Att` (struct :`Name` "Dimmer")) (`BlueprintMapLibrary.Map_Find` `DMX Att`) (`BlueprintMapLibrary.Map_Find` `DMX Att` (struct :`Name` "Tint")) (`BlueprintMapLibrary.Map_Find` `DMX Att` (struct :`Name` "CrossFadetoColor")) (`BlueprintMapLibrary.Map_Find` `DMX Att` (struct :`Name` "Red")) (`BlueprintMapLibrary.Map_Find` `DMX Att` (struct :`Name` "Green")) (`BlueprintMapLibrary.Map_Find` `DMX Att` (struct :`Name` "Blue")) (`BlueprintMapLibrary.Map_Find` `DMX Att` (struct :`Name` "White")) (`BlueprintMapLibrary.Map_Find` `DMX Att` (struct :`Name` "Velocity")) (`BlueprintMapLibrary.Map_Find` `DMX Att` (struct :`Name` "Effects")) (`BlueprintMapLibrary.Map_Find` `DMX Att` (struct :`Name` "Shutter")) (`BlueprintMapLibrary.Map_Find` `DMX Att` (struct :`Name` "Dummy"))))

(fn `M90Functions`
  (params (TiltBody :type "Float (double-precision)") (SetTemp :type Boolean) (Color :type "LinearColor Structure") (Intensity :type "Float (double-precision)") (Kelvin :type String) (ShadowBias :type "Float (double-precision)") (LeafRight :type "Float (double-precision)") (LeafLeft :type "Float (double-precision)") (LeafTop :type "Float (double-precision)") (LeafBottom :type "Float (double-precision)") (Lens :type "/TechvizSharedAssets/StudioLightingKit/BluePrints/ENU_M90_Lens Enum" :default "NewEnumerator0") (`Hide Hang` :type Boolean) (`Hide BarnDoor` :type Boolean))
  (bind _hang (`self.Hang`))
  (bind _m90_leafsframe (`self.M90_LeafsFrame`))
  (bind _pointlight (`self.PointLight`))
  (bind _spotlight (`self.SpotLight`))
  (bind _m90_lens (`self.M90_Lens`))
  (`|ExecutionSequence`
    (:`then_0`
      (if SetTemp
        (bind _rgba (`/TechvizSharedAssets/StudioLightingKit/BluePrints/BP_FunctionLibrary.KelvinStringsToRGBA` Kelvin))
        (set `self.CurrentColor` _rgba)
        (else
          (set `self.CurrentColor` Color)))
      (`PrimitiveComponent.SetCustomPrimitiveDataVector3` _m90_lens 0 (`KismetMathLibrary.Conv_LinearColorToVector` (`self.CurrentColor`)))
      (`PrimitiveComponent.SetCustomPrimitiveDataFloat` _m90_lens 4 (/ Intensity 100.0))
      (`LightComponent.SetIntensity` _spotlight Intensity)
      (`LightComponent.SetLightColor` _spotlight (`self.CurrentColor`) true)
      (`LightComponent.SetShadowBias` _spotlight ShadowBias)
      (`LightComponent.SetShadowBias` _spotlight ShadowBias)
      (`LightComponent.SetIntensity` _pointlight (/ Intensity 1000.0))
      (`LightComponent.SetLightColor` _pointlight (`self.CurrentColor`) true)
      (`self.SetLensArray`
        (:`_`
          (`LightComponent.SetIESTexture` _spotlight (`|GetArrayItem` (`self.LensArray`) (`KismetMathLibrary.Conv_ByteToInt` Lens))))))
    (:`then_1`
      (`SceneComponent.K2_SetRelativeRotation` (`self.body`) (`KismetMathLibrary.MakeRotator` 0.0 TiltBody) false false)
      (`SceneComponent.K2_SetRelativeRotation` (`self.M90_LeafRight`) (`KismetMathLibrary.MakeRotator` 0.0 0.0 LeafRight) false false)
      (`SceneComponent.K2_SetRelativeRotation` (`self.M90_LeafLeft`) (`KismetMathLibrary.MakeRotator` 0.0 0.0 LeafLeft) false false)
      (`SceneComponent.K2_SetRelativeRotation` (`self.M90_LeafTop`) (`KismetMathLibrary.MakeRotator` 0.0 LeafTop) false false)
      (`SceneComponent.K2_SetRelativeRotation` (`self.M90_LeafBottom`) (`KismetMathLibrary.MakeRotator` 0.0 LeafBottom) false false)
      (`SceneComponent.SetHiddenInGame` _m90_leafsframe `Hide BarnDoor` false)
      (`SceneComponent.SetVisibility` _m90_leafsframe (not `Hide BarnDoor`) true)
      (`SceneComponent.SetHiddenInGame` _hang `Hide Hang` false)
      (`SceneComponent.SetVisibility` _hang (not `Hide Hang`) false))))

(fn `UserConstructionScript`
  (`self.M90Functions` (`self.TiltBody`) (`self.Set Temp`) (`self.Color`) (`self.Intensity`) (`|GetEnumeratorNameAsString` (`self.Kelvin`)) (`self.ShadowBias`) (`self.LeafRight`) (`self.LeafLeft`) (`self.LeafTop`) (`self.LeafBottom`) (`self.Lens`) (`self.Hide Hang`) (`self.Hide BarnDoor`)))