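; BP_Plug is a D1 studio prop whose plug material previews an LED wall look in Grid, Check Pattern or N Display mode.
; The Construction Script switches on LEDWallColorMode, assigns the D1_Plug slot material, then creates a dynamic instance on element 2.
; Plug variables drive its colors, opacities and light power, plus an optional number in Check Pattern; N Display sets only wall color.
; The event graph is empty.
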(fn `UserConstructionScript`
  (bind _staticmesh (`self.StaticMesh`))
  (switch `/TechvizSharedAssets/Asset/Prop/Studio_v02/D1_Studio_LiDAR/BP/Enum/LED_Wall_Mode` (`self.LED_Wall_Color_Mode`)
    (:`NewEnumerator0`
      (`PrimitiveComponent.SetMaterialByName` _staticmesh "D1_Plug" "/TechvizSharedAssets/Asset/Prop/Studio_v02/D1_Studio_LiDAR/Material/LED_Material/D1_Plug_Grid.D1_Plug_Grid")
      (bind _returnvalue (`PrimitiveComponent.CreateDynamicMaterialInstance` _staticmesh 2 "/TechvizSharedAssets/Asset/Prop/Studio_v02/D1_Studio_LiDAR/Material/Material_inst/D1_Plug_Inst.D1_Plug_Inst" "None"))
      (`MaterialInstanceDynamic.SetVectorParameterValue` _returnvalue "Wall_Color" (`self.Plug_Wall_Color`))
      (`MaterialInstanceDynamic.SetVectorParameterValue` _returnvalue "Grid_Color" (`self.Plug_Grid_Color`))
      (`MaterialInstanceDynamic.SetScalarParameterValue` _returnvalue "LED_Wall_Opacity" (`self.Plug_Wall_Opacity`))
      (`MaterialInstanceDynamic.SetScalarParameterValue` _returnvalue "Grid_Opacity" (`self.Plug_Grid_Opacity`))
      (`MaterialInstanceDynamic.SetScalarParameterValue` _returnvalue "Light_Power" (`self.Plug_Power_Intensity`)))
    (:`NewEnumerator1`
      (`PrimitiveComponent.SetMaterialByName` _staticmesh "D1_Plug" "/TechvizSharedAssets/Asset/Prop/Studio_v02/D1_Studio_LiDAR/Material/LED_Material/D1_Plug_ColoredGrid.D1_Plug_ColoredGrid")
      (bind _returnvalue_2 (`PrimitiveComponent.CreateDynamicMaterialInstance` _staticmesh 2 "/TechvizSharedAssets/Asset/Prop/Studio_v02/D1_Studio_LiDAR/Material/Material_inst/D1_Plug_ColoredGrid_Inst.D1_Plug_ColoredGrid_Inst" "None"))
      (`MaterialInstanceDynamic.SetVectorParameterValue` _returnvalue_2 "Color_01" (`self.Plug_Wall_Color`))
      (`MaterialInstanceDynamic.SetVectorParameterValue` _returnvalue_2 "Color_02" (`self.Plug_Check_Pattern_Color`))
      (`MaterialInstanceDynamic.SetScalarParameterValue` _returnvalue_2 "LED_Wall_Opacity" (`self.Plug_Wall_Opacity`))
      (`MaterialInstanceDynamic.SetScalarParameterValue` _returnvalue_2 "Grid_Opacity" (`self.Plug_Grid_Opacity`))
      (`MaterialInstanceDynamic.SetScalarParameterValue` _returnvalue_2 "Light_Power" (`self.Plug_Power_Intensity`))
      (if (`self.Plug_Number_On/Off`)
        (`MaterialInstanceDynamic.SetScalarParameterValue` _returnvalue_2 "LogoScale" (`self.Plug_Number_Scale`))
        (`MaterialInstanceDynamic.SetVectorParameterValue` _returnvalue_2 "Logo_Color" (`self.Plug_Number_Color`))
        (else
          (`MaterialInstanceDynamic.SetScalarParameterValue` _returnvalue_2 "LogoScale" 0.0))))
    (:`NewEnumerator2`
      (`PrimitiveComponent.SetMaterialByName` _staticmesh "D1_Plug" "/TechvizSharedAssets/Asset/Prop/Studio_v02/D1_Studio_LiDAR/Material/LED_Material/D1_Plug_JustColor.D1_Plug_JustColor")
      (bind _returnvalue_3 (`PrimitiveComponent.CreateDynamicMaterialInstance` _staticmesh 2 "/TechvizSharedAssets/Asset/Prop/Studio_v02/D1_Studio_LiDAR/Material/LED_Material/D1_Plug_JustColor.D1_Plug_JustColor" "None"))
      (`MaterialInstanceDynamic.SetVectorParameterValue` _returnvalue_3 "Wall_Color" (`self.Plug_Wall_Color`)))))