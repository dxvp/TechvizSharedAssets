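; BP_Rail_v01 is a modular rail prop that builds a straight run toward the InLocation offset in its construction script.
; It divides the horizontal distance, less 100 units, by MeshWidth, adds repeated meshes along the Rail's X axis, and yaws the Rail toward that point.
; A flag widens the rail 1.67x, and a flat TextRender at the endpoint shows segment count and length at two meters each.
; The event graph is empty.
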(fn `UserConstructionScript`
  (bind _returnvalue (`self.K2_GetActorLocation`))
  (bind (_in_location_x _in_location_y) (`KismetMathLibrary.BreakVector` (`self.In Location`)))
  (bind _rail (`self.Rail`))
  (bind _yaw (.yaw (`KismetMathLibrary.FindLookAtRotation` _returnvalue (+ _returnvalue (`self.In Location`)))))
  (bind _returnvalue_2 (`KismetMathLibrary.Round` (/ (- (`KismetMathLibrary.VSize` (* (`self.In Location`) (1.0 1.0 0.0))) 100.0) (`self.Mesh width`))))
  (bind _returnvalue_3 (- _returnvalue_2 1))
  (`StaticMeshComponent.SetStaticMesh` _rail (`self.타깃`))
  (if (`self.60cm/1m (Width)`)
    (`SceneComponent.K2_SetRelativeTransform` _rail (`KismetMathLibrary.MakeTransform` (0.0 0.0 0.0) (struct) (1.0 1.67 1.0)) false false)
    (else
      (`SceneComponent.K2_SetRelativeTransform` _rail (`KismetMathLibrary.MakeTransform` (0.0 0.0 0.0)) false false)))
  (if (> _returnvalue_3 0)
    (for _index (range 1 (+ _returnvalue_3 1))
      (bind _returnvalue_4 (`AddComponent|NODE_AddStaticMeshComponent-2` :`bManualAttachment` true))
      (`SceneComponent.K2_AttachTo` _returnvalue_4 (`self.Rail`) "None" "KeepWorldPosition" true)
      (`SceneComponent.K2_SetRelativeTransform` _returnvalue_4 (`KismetMathLibrary.MakeTransform` (`KismetMathLibrary.MakeVector` (* _index (`self.Mesh width`)))) false false)
      (`StaticMeshComponent.SetStaticMesh` _returnvalue_4 (`self.타깃`))))
  (`SceneComponent.K2_SetWorldRotation` (`self.Rail`) (`KismetMathLibrary.MakeRotator` 0.0 0.0 _yaw) false false)
  (`SceneComponent.K2_SetRelativeTransform` (`self.TextRender`) (`KismetMathLibrary.MakeTransform` (`KismetMathLibrary.MakeVector` _in_location_x _in_location_y 1.0) (`KismetMathLibrary.MakeRotator` 0.0 90.0 _yaw) (`KismetMathLibrary.Conv_DoubleToVector` (`self.Text Size`))) false false)
  (`TextRenderComponent.K2_SetText` (`self.TextRender`) (`KismetTextLibrary.Conv_StringToText` (`KismetStringLibrary.Concat_StrStr` (`KismetTextLibrary.Conv_TextToString` (`KismetTextLibrary.Conv_IntToText` _returnvalue_2)) "(" (`KismetStringLibrary.Conv_IntToString` (* _returnvalue_2 2)) "m" ")"))))