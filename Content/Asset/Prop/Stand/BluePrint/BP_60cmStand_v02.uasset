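; Procedural 60cm stand prop, a generated dynamic mesh actor that rebuilds its shape and dimension labels from exposed variables.
; On rebuild it copies the 60cmStand static mesh and plane-cuts it to length in 122-unit steps.
; Geometry Script boolean subtractions then carve four box sections sized by L, M, R and RR.
; Text renders show the overall and per-section lengths, with section labels repositioned and shown or hidden to match the cuts.
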(event Events|EventOnRebuildGeneratedMesh
  (params (TargetMesh :type Dynamic%20Mesh%20Object%20Reference))
  (bind _m (Variables|Default|GetM))
  (bind _빼기 (Variables|Default|Get빼기))
  (bind _r (Variables|Default|GetR))
  (bind _빼기_2 (Variables|Default|Get빼기))
  (bind _text_scale (Variables|Default|GetText%20Scale))
  (bind _textrender4 (Variables|Default|GetTextRender4))
  (bind _l (Variables|Default|GetL))
  (bind _cut_frame_location_x (Variables|Default|GetCut%20Frame%20Location%20X))
  (bind _빼기_3 (Variables|Default|Get빼기))
  (bind _returnvalue (Math|Conversions|ToVector(Float) _text_scale))
  (bind _returnvalue_2 (* _cut_frame_location_x 122))
  (bind _returnvalue_3 (* _l _빼기))
  (bind _returnvalue_4 (* _m _빼기_2))
  (bind _returnvalue_5 (* _r _빼기_3))
  (bind _returnvalue_6 (* _returnvalue_5 2.0))
  (bind _returnvalue_7 (* _returnvalue_3 2.0))
  (bind _returnvalue_8 (* _returnvalue_4 2.0))
  (bind _returnvalue_9 (- _returnvalue_2 1056.0))
  (bind _returnvalue_10 (GeometryScript|StaticMesh|CopyMeshFromStaticMesh :FromStaticMeshAsset "/TechvizSharedAssets/Asset/Prop/Stand/Component/60cmStand.60cmStand" :ToDynamicMesh TargetMesh :Debug 0)
    (:Success
      (bind _returnvalue_11 (Class|GeometryScriptLibraryMeshBooleanFunctions|ApplyMeshPlaneCut :TargetMesh _returnvalue_10 :CutFrame (Math|Transform|MakeTransform (Math|Vector|MakeVector (+ (* _returnvalue_2 -1.0) 621.0) 0.0 0.0) "-90.000000, 0, 0" "1.000000,1.000000,1.000000") :Debug 0))
      (Rendering|Material|SetMaterial (Variables|DynamicMeshActor|GetDynamicMeshComponent) 0 (Variables|Default|GetMaterial))
      (Rendering|Components|TextRender|SetText (Variables|Default|GetTextRender) (Utilities|Text|ToText(String) (Utilities|String|Append "Length: " (Utilities|String|ToString(Integer) (|(floor((abs(x)))) _returnvalue_9)))))
      (Utilities|FlowControl|Sequence
        (:then_0
          (bind _returnvalue_12 (DynamicMeshActor|AllocateComputeMesh))
          (bind _returnvalue_13 (Class|GeometryScriptLibraryMeshPrimitiveFunctions|AppendBox :TargetMesh _returnvalue_12 :Transform (Math|Transform|MakeTransform (Math|Vector|MakeVector (+ 0.0 (- _returnvalue_3 477.0)) (Variables|Default|GetL_point) -0.1) "0, 0, 0" (Math|Vector|MakeVector (* _returnvalue_3 0.02) 2.44 2.0)) :Debug 0))
          (bind _returnvalue_14 (GeometryScript|Booleans|ApplyMeshBoolean :TargetMesh _returnvalue_11 :ToolMesh _returnvalue_13 :Operation "Subtract" :Debug 0))
          (bind _returnvalue_15 (DynamicMeshActor|AllocateComputeMesh))
          (bind _returnvalue_16 (Class|GeometryScriptLibraryMeshPrimitiveFunctions|AppendBox :TargetMesh _returnvalue_15 :Transform (Math|Transform|MakeTransform (Math|Vector|MakeVector (+ 0.0 (- _returnvalue_4 477.0)) (Variables|Default|GetM_point) -0.1) "0, 0, 0" (Math|Vector|MakeVector (* _returnvalue_4 0.02) 2.44 2.0)) :Debug 0))
          (bind _returnvalue_17 (GeometryScript|Booleans|ApplyMeshBoolean :TargetMesh _returnvalue_14 :ToolMesh _returnvalue_16 :Operation "Subtract" :Debug 0))
          (bind _returnvalue_18 (DynamicMeshActor|AllocateComputeMesh))
          (bind _returnvalue_19 (Class|GeometryScriptLibraryMeshPrimitiveFunctions|AppendBox :TargetMesh _returnvalue_18 :Transform (Math|Transform|MakeTransform (Math|Vector|MakeVector (+ 0.0 (- _returnvalue_5 477.0)) (Variables|Default|GetR_point) -0.1) "0, 0, 0" (Math|Vector|MakeVector (* _returnvalue_5 0.02) 2.44 1.0)) :Debug 0))
          (bind _returnvalue_20 (GeometryScript|Booleans|ApplyMeshBoolean :TargetMesh _returnvalue_17 :ToolMesh _returnvalue_19 :Operation "Subtract" :Debug 0))
          (if (>= 2 (Variables|Default|GetRR))
            (Variables|Default|SetNewVar_0 1)
            (else
              (Variables|Default|SetNewVar_0 2)))
          (bind _returnvalue_21 (DynamicMeshActor|AllocateComputeMesh))
          (bind _returnvalue_22 (Class|GeometryScriptLibraryMeshPrimitiveFunctions|AppendBox :TargetMesh _returnvalue_21 :Transform (Math|Transform|MakeTransform (Math|Vector|MakeVector (+ 0.0 (- (* (+ (Variables|Default|GetRR) (Variables|Default|GetNewVar_0)) 122.0) 599.0)) (Variables|Default|GetRR_point) -0.1) "0, 0, 0" (Math|Vector|MakeVector (* (* (+ (Variables|Default|GetRR) (Variables|Default|GetNewVar_0)) 122.0) 0.02) 0.5 1.0)) :Debug 0))
          (GeometryScript|Booleans|ApplyMeshBoolean :TargetMesh _returnvalue_20 :ToolMesh _returnvalue_22 :Operation "Subtract" :Debug 0))
        (:then_1
          (Transformation|SetRelativeTransform (Variables|Default|GetTextRender1) (Math|Transform|MakeTransform (Math|Vector|MakeVector (+ _returnvalue_7 -5e+02) -2.7e+02 1.0) "90.000000,180.000000, 0" _returnvalue) false false)
          (Transformation|SetRelativeTransform (Variables|Default|GetTextRender2) (Math|Transform|MakeTransform (Math|Vector|MakeVector (+ _returnvalue_8 -5e+02) -25.0 1.0) "90.000000,180.000000, 0" _returnvalue) false false)
          (Transformation|SetRelativeTransform (Variables|Default|GetTextRender3) (Math|Transform|MakeTransform (Math|Vector|MakeVector (+ _returnvalue_6 -5e+02) 225.0 1.0) "90.000000,180.000000, 0" _returnvalue) false false)
          (Transformation|SetRelativeTransform (Variables|Default|GetTextRender4) (Math|Transform|MakeTransform (Math|Vector|MakeVector (+ (* (* (+ (Variables|Default|GetRR) (Variables|Default|GetNewVar_0)) 122.0) 2.0) -6e+02) 4.2e+02 1.0) "90.000000,90.000000, 0" _returnvalue) false false))
        (:then_2
          (if (> 1 (Variables|Default|GetCut%20Frame%20Location%20X))
            (Variables|Default|SetNewVar_1 0)
            (else
              (Variables|Default|SetNewVar_1 42)))
          (Rendering|SetVisibility (Variables|Default|GetTextRender1) (< (Variables|Default|GetCut%20Frame%20Location%20X) (|((abs((x-8)))+1) (Math|Conversions|ToFloat(Integer) (Variables|Default|GetL)))) false)
          (Rendering|SetVisibility (Variables|Default|GetTextRender2) (< (Variables|Default|GetCut%20Frame%20Location%20X) (|((abs((x-8)))+1) (Math|Conversions|ToFloat(Integer) (Variables|Default|GetM)))) false)
          (Rendering|SetVisibility (Variables|Default|GetTextRender3) (< (Variables|Default|GetCut%20Frame%20Location%20X) (|((abs((x-8)))+1) (Math|Conversions|ToFloat(Integer) (Variables|Default|GetR)))) false))
        (:then_3
          (CallFunction|TextFunction (Variables|Default|GetTextRender1) _returnvalue_7 "L:" (+ (* _returnvalue_9 -1.0) (Variables|Default|GetNewVar_1)))
          (CallFunction|TextFunction (Variables|Default|GetTextRender2) _returnvalue_8 "M:" (+ (* _returnvalue_9 -1.0) (Variables|Default|GetNewVar_1)))
          (CallFunction|TextFunction (Variables|Default|GetTextRender3) _returnvalue_6 "R:" (+ (* _returnvalue_9 -1.0) (Variables|Default|GetNewVar_1)))
          (CallFunction|TextFunction _textrender4 (* (* (+ (Variables|Default|GetRR) (Variables|Default|GetNewVar_0)) 122.0) 2.0) "RR:" (+ (+ (* _returnvalue_9 -1.0) (Variables|Default|GetNewVar_1)) 122.0))
          (Rendering|SetVisibility _textrender4 (>= 2 (Variables|Default|GetRR)) false)
          (Rendering|SetVisibility (Variables|Default|GetTextRender4) (< (/ (Variables|Default|GetCut%20Frame%20Location%20X) 3) (|(abs((x-3))) (Math|Conversions|ToFloat(Integer) (Variables|Default|GetRR)))) false))))))

(fn ConstructionScript)

(fn TextFunction
  (params (textTarget :type Text%20Render%20Component%20Object%20Reference) (result :type Float%20%28double-precision%29) (덧붙이기 :type String) (value :type Float%20%28double-precision%29))
  (Rendering|Components|TextRender|SetText textTarget (Utilities|Text|ToText(String) (Utilities|String|Append 덧붙이기 (Utilities|String|ToString(Integer) (|(floor((abs(x)))) (- result value)))))))