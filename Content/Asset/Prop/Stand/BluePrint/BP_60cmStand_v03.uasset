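; Generated dynamic mesh prop that builds a parametric 60cm stand from a static mesh, trimmed to an adjustable length.
; On rebuild it copies the mesh, plane-cuts it along X, applies the material and displays the length.
; BooleanCalculator then sizes boxes from the L, M, R and RR values, which are boolean-subtracted to carve four sections.
; Logic for positioning, filling and hiding per-section text labels exists but is disconnected.
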(event Events|EventOnRebuildGeneratedMesh
  (params (TargetMesh :type Dynamic%20Mesh%20Object%20Reference))
  (bind _cut_frame_location_x (Variables|Default|GetCut%20Frame%20Location%20X))
  (bind _returnvalue (* _cut_frame_location_x 122))
  (bind _returnvalue_2 (- _returnvalue 1056.0))
  (Class|DynamicMeshComponent|EnableComplexasSimpleCollision (Variables|DynamicMeshActor|GetDynamicMeshComponent))
  (bind _returnvalue_3 (GeometryScript|StaticMesh|CopyMeshFromStaticMesh :FromStaticMeshAsset "/TechvizSharedAssets/Asset/Prop/Stand/Component/60cm_Stand_v03.60cm_Stand_v03" :ToDynamicMesh TargetMesh :Debug 0)
    (:Success
      (bind _output_get (Variables|Default|SetTarget%20Mesh _returnvalue_3))
      (Class|GeometryScriptLibraryMeshBooleanFunctions|ApplyMeshPlaneCut :TargetMesh _output_get :CutFrame (Math|Transform|MakeTransform (Math|Vector|MakeVector (+ (* _returnvalue -1.0) 712.226) 0.0 0.0) "-90.000000, 0, 0" "1.000000,1.000000,1.000000") :Debug 0)
      (Rendering|Material|SetMaterial (Variables|DynamicMeshActor|GetDynamicMeshComponent) 0 (Variables|Default|GetMaterial))
      (Rendering|Components|TextRender|SetText (Variables|Default|GetTextRender) (Utilities|Text|ToText(String) (Utilities|String|Append "Length: " (Utilities|String|ToString(Integer) (|(floor((abs(x)))) _returnvalue_2)))))
      (Variables|Default|SetsubtractedCutFrame _returnvalue_2)
      (Utilities|FlowControl|Sequence
        (:then_0
          (Utilities|FlowControl|Sequence
            (:then_0
              (bind (_transformlacation_x _offsetscale_trnasformscalex_ _texttransform) (CallFunction|BooleanCalculator (Variables|Default|GetL) 61.0 349.361))
              (Variables|Default|SettextVal_L _texttransform)
              (bind _returnvalue_4 (DynamicMeshActor|AllocateComputeMesh))
              (bind _returnvalue_5 (Class|GeometryScriptLibraryMeshPrimitiveFunctions|AppendBox :TargetMesh _returnvalue_4 :Transform (Math|Transform|MakeTransform (Math|Vector|MakeVector _transformlacation_x (Variables|Default|GetL_point) -0.1) "0, 0, 0" (Math|Vector|MakeVector _offsetscale_trnasformscalex_ 2.44 2.0)) :Debug 0))
              (GeometryScript|Booleans|ApplyMeshBoolean :TargetMesh (Variables|Default|GetTarget%20Mesh) :ToolMesh _returnvalue_5 :Operation "Subtract" :Debug 0))
            (:then_1
              (bind (_transformlacation_x_2 _offsetscale_trnasformscalex__2 _texttransform_2) (CallFunction|BooleanCalculator (Variables|Default|GetM) 61.0 349.361))
              (Variables|Default|SettextVal_M _texttransform_2)
              (bind _returnvalue_6 (DynamicMeshActor|AllocateComputeMesh))
              (bind _returnvalue_7 (Class|GeometryScriptLibraryMeshPrimitiveFunctions|AppendBox :TargetMesh _returnvalue_6 :Transform (Math|Transform|MakeTransform (Math|Vector|MakeVector _transformlacation_x_2 (Variables|Default|GetM_point) -0.1) "0, 0, 0" (Math|Vector|MakeVector _offsetscale_trnasformscalex__2 2.44 2.0)) :Debug 0))
              (GeometryScript|Booleans|ApplyMeshBoolean :TargetMesh (Variables|Default|GetTarget%20Mesh) :ToolMesh _returnvalue_7 :Operation "Subtract" :Debug 0))
            (:then_2
              (bind (_transformlacation_x_3 _offsetscale_trnasformscalex__3 _texttransform_3) (CallFunction|BooleanCalculator (Variables|Default|GetR) 61.0 349.361))
              (Variables|Default|SettextVal_R _texttransform_3)
              (bind _returnvalue_8 (DynamicMeshActor|AllocateComputeMesh))
              (bind _returnvalue_9 (Class|GeometryScriptLibraryMeshPrimitiveFunctions|AppendBox :TargetMesh _returnvalue_8 :Transform (Math|Transform|MakeTransform (Math|Vector|MakeVector _transformlacation_x_3 (Variables|Default|GetR_point) -0.1) "0, 0, 0" (Math|Vector|MakeVector _offsetscale_trnasformscalex__3 2.44 1.0)) :Debug 0))
              (GeometryScript|Booleans|ApplyMeshBoolean :TargetMesh (Variables|Default|GetTarget%20Mesh) :ToolMesh _returnvalue_9 :Operation "Subtract" :Debug 0))
            (:then_3
              (if (>= 3 (Variables|Default|GetRR))
                (Variables|Default|SetNewVar_0 1)
                (else
                  (Variables|Default|SetNewVar_0 2)))
              (bind (_transformlacation_x_4 _offsetscale_trnasformscalex__4 _texttransform_4) (CallFunction|BooleanCalculator (+ (Variables|Default|GetRR) (Variables|Default|GetNewVar_0)) 122.0 593.361))
              (Variables|Default|SettextVal_RR _texttransform_4)
              (bind _returnvalue_10 (DynamicMeshActor|AllocateComputeMesh))
              (bind _returnvalue_11 (Class|GeometryScriptLibraryMeshPrimitiveFunctions|AppendBox :TargetMesh _returnvalue_10 :Transform (Math|Transform|MakeTransform (Math|Vector|MakeVector _transformlacation_x_4 (Variables|Default|GetRR_point) -0.1) "0, 0, 0" (Math|Vector|MakeVector _offsetscale_trnasformscalex__4 0.5 1.0)) :Debug 0))
              (GeometryScript|Booleans|ApplyMeshBoolean :TargetMesh (Variables|Default|GetTarget%20Mesh) :ToolMesh _returnvalue_11 :Operation "Subtract" :Debug 0))))))))

(fn ConstructionScript)

(fn TextFunction
  (params (textTarget :type Text%20Render%20Component%20Object%20Reference) (result :type Float%20%28double-precision%29) (덧붙이기 :type String) (value :type Float%20%28double-precision%29))
  (Rendering|Components|TextRender|SetText textTarget (Utilities|Text|ToText(String) (Utilities|String|Append 덧붙이기 (Utilities|String|ToString(Integer) (|(floor((abs(x)))) (- result value)))))))

(fn BooleanCalculator
  (params (What%20position :type Integer) (subtractLangth :type Float%20%28double-precision%29) (Offset :type Float%20%28double-precision%29))
  (bind _returnvalue (* What%20position subtractLangth))
  (return (- _returnvalue Offset) (* _returnvalue 0.02) (* _returnvalue 2.0)))