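; Generated-mesh prop for a 60cm stand with adjustable length and a text readout of that length.
; On rebuild it copies the static stand mesh into the dynamic mesh, plane-cuts it at a scaled CutFrameLocationX and applies the material.
; It then boolean-subtracts a box sized by L and placed from the cut position and LPoint.
; A separate TextFunction formats an offset value as prefixed, floored absolute text.
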(event Events|EventOnRebuildGeneratedMesh
  (params (TargetMesh :type Dynamic%20Mesh%20Object%20Reference))
  (bind _빼기 (Variables|Default|Get빼기))
  (bind _l (Variables|Default|GetL))
  (bind _cut_frame_location_x (Variables|Default|GetCut%20Frame%20Location%20X))
  (bind _returnvalue (* _cut_frame_location_x 122))
  (bind _returnvalue_2 (* _l _빼기))
  (bind _returnvalue_3 (GeometryScript|StaticMesh|CopyMeshFromStaticMesh :FromStaticMeshAsset "/TechvizSharedAssets/Asset/Prop/stand/MASH/60cm_Stand.60cm_Stand" :ToDynamicMesh TargetMesh :Debug 0)
    (:Success
      (Class|GeometryScriptLibraryMeshBooleanFunctions|ApplyMeshPlaneCut :TargetMesh _returnvalue_3 :CutFrame (Math|Transform|MakeTransform (Math|Vector|MakeVector (- _returnvalue 477.0) 0.0 0.0) "90.000000, 0, 0" "1.000000,1.000000,1.000000") :Debug 0)
      (Rendering|Material|SetMaterial (Variables|DynamicMeshActor|GetDynamicMeshComponent) 0 (Variables|Default|GetMaterial))
      (Rendering|Components|TextRender|SetText (Variables|Default|GetTextRender) (Utilities|Text|ToText(String) (Utilities|String|Append "Length: " (Utilities|String|ToString(Integer) (|(floor((abs(x)))) (- _returnvalue 1056.0))))))
      (bind _returnvalue_4 (DynamicMeshActor|AllocateComputeMesh))
      (bind _returnvalue_5 (Class|GeometryScriptLibraryMeshPrimitiveFunctions|AppendBox :TargetMesh _returnvalue_4 :Transform (Math|Transform|MakeTransform (Math|Vector|MakeVector (+ _returnvalue (- _returnvalue_2 477.0)) (Variables|Default|GetL_point) -0.1) "0, 0, 0" (Math|Vector|MakeVector (* _returnvalue_2 0.02) 2.44 2.0)) :Debug 0))
      (GeometryScript|Booleans|ApplyMeshBoolean :ToolMesh _returnvalue_5 :Operation "Subtract" :Debug 0))))

(fn ConstructionScript)

(fn TextFunction
  (params (textTarget :type Text%20Render%20Component%20Object%20Reference) (result :type Float%20%28double-precision%29) (덧붙이기 :type String) (value :type Float%20%28double-precision%29))
  (Rendering|Components|TextRender|SetText textTarget (Utilities|Text|ToText(String) (Utilities|String|Append 덧붙이기 (Utilities|String|ToString(Integer) (|(floor((abs(x)))) (- result value)))))))