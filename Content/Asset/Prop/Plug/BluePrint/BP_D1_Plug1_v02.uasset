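; Generated dynamic mesh plug prop that carves a grid-sized rectangular piece out of a stage static mesh.
; On rebuild, it copies the mesh and uses Geometry Script to boolean-intersect it with a box positioned by LeftRight/UpDown and sized by Width/Hight.
; Two text renders display the piece's width and height in cells, reduced when the box overruns the 9 by 8 grid.
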(event `self.OnRebuildGeneratedMesh`
  (params (TargetMesh :type "DynamicMesh Object Reference"))
  (bind _width (`self.Width`))
  (bind _left___right (`self.Left & Right`))
  (bind _up___down (`self.Up & Down`))
  (bind _hight (`self.Hight`))
  (bind _textrender (`self.TextRender`))
  (bind _textrender1 (`self.TextRender1`))
  (bind (_returnvalue_x _returnvalue_y) (`KismetMathLibrary.BreakVector` (* _width (0.5 0.5 0.5))))
  (bind _returnvalue (* _hight 0.5))
  (bind _returnvalue_2 (* _width 0.5))
  (bind _returnvalue_3 (+ _up___down _hight))
  (bind _returnvalue_4 (+ _left___right _width))
  (bind _returnvalue_5 (- _hight _returnvalue_3))
  (bind _returnvalue_6 (- _width _returnvalue_4))
  (bind _returnvalue_7 (`GeometryScriptLibrary_StaticMeshFunctions.CopyMeshFromStaticMesh` "/TechvizSharedAssets/Asset/Prop/Plug/MESH/D1_Stage_polySurface823.D1_Stage_polySurface823" TargetMesh (struct) (struct) null)
    (:`Success`
      (`PrimitiveComponent.SetMaterial` (`self.DynamicMeshComponent`) 0 (`self.Material`))
      (bind _returnvalue_8 (`self.AllocateComputeMesh`))
      (bind _returnvalue_9 (`GeometryScriptLibrary_MeshPrimitiveFunctions.AppendBox` _returnvalue_8 (struct) (`KismetMathLibrary.MakeTransform` (`KismetMathLibrary.MakeVector` (+ (+ (* _left___right 50) (+ -175.0 0.0)) (- (* 50.0 _returnvalue_2) 50.0)) (+ 0.0 1.0) (+ (+ (* _up___down 50) (+ 0.0 98.5)) (- (* 50.0 _returnvalue) 50.0))) (struct) (`KismetMathLibrary.MakeVector` _returnvalue_2 _returnvalue_y _returnvalue)) 100.0 100.0 100.0 0 0 0 "Center" null))
      (`GeometryScriptLibrary_MeshBooleanFunctions.ApplyMeshBoolean` _returnvalue_7 (struct) _returnvalue_9 (struct) "Intersection" (struct) null)
      (`|ExecutionSequence`
        (:`then_0`
          (if (< _returnvalue_4 10)
            (`TextRenderComponent.K2_SetText` _textrender (`KismetTextLibrary.Conv_IntToText` _width))
            (else
              (`TextRenderComponent.K2_SetText` _textrender (`KismetTextLibrary.Conv_IntToText` _returnvalue_6))
              (if (<= _returnvalue_6 0)
                (`TextRenderComponent.K2_SetText` _textrender (`KismetTextLibrary.Conv_IntToText` (+ _returnvalue_6 9)))))))
        (:`then_1`
          (if (< _returnvalue_3 9)
            (`TextRenderComponent.K2_SetText` _textrender1 (`KismetTextLibrary.Conv_IntToText` _hight))
            (else
              (`TextRenderComponent.K2_SetText` _textrender1 (`KismetTextLibrary.Conv_IntToText` _returnvalue_5))
              (if (<= _returnvalue_5 0)
                (`TextRenderComponent.K2_SetText` _textrender1 (`KismetTextLibrary.Conv_IntToText` (+ _returnvalue_5 8)))))))))))

(fn `UserConstructionScript`)