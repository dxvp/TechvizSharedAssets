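; Mini jib camera crane prop, posed from pan, tilt, arm length and head rotation variables, that carries a linked Cam actor.
; One Kernal function runs on construction and Tick, setting the wheel layout and crane part transforms.
; The head and supports counter or follow the arm tilt, while length slides front and back sections and spins the handle.
; Cam snaps to the head mount's world position, its yaw following pan and head rotation.
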(event `self.ReceiveTick`
  (params (DeltaSeconds :type "Float (single-precision)"))
  (`self.Kernal`))

(fn `Kernal`
  (bind _returnvalue (`self.GetTransform`))
  (bind _langth (`self.Langth`))
  (bind _staticmesh (`self.StaticMesh`))
  (bind (_cam_position_x _cam_position_y _cam_position_z) (`KismetMathLibrary.BreakVector` (`self.Cam Position`)))
  (bind _horizontal (`self.Horizontal`))
  (bind _returnvalue_location (`KismetMathLibrary.BreakTransform` (`SceneComponent.K2_GetComponentToWorld` (`self.StaticMesh1`))))
  (`|ExecutionSequence`
    (:`then_0`
      (`SceneComponent.K2_SetWorldTransform` (`self.bodyMain`) (`KismetMathLibrary.MakeTransform` (.location _returnvalue) (`KismetMathLibrary.MakeRotator` (+ (.roll (.rotation _returnvalue)) 90.0) (.pitch (.rotation _returnvalue)) (.yaw (.rotation _returnvalue)))) false false))
    (:`then_1`
      (if (`self.60cm/1m`)
        (`|ExecutionSequence`
          (:`then_0`
            (`SceneComponent.K2_SetRelativeLocation` (`self.wheel01`) (10.0 0.0 10.0) false false))
          (:`then_1`
            (`SceneComponent.K2_SetRelativeLocation` (`self.wheel02`) (-10.0 0.0 10.0) false false))
          (:`then_2`
            (`SceneComponent.K2_SetRelativeLocation` (`self.wheel03`) (10.0 0.0 -10.0) false false))
          (:`then_3`
            (`SceneComponent.K2_SetRelativeLocation` (`self.wheel04`) (-10.0 0.0 -10.0) false false)))))
    (:`then_2`
      (`|ExecutionSequence`
        (:`then_0`
          (`SceneComponent.K2_SetRelativeRotation` (`self.crainBody`) (`KismetMathLibrary.MakeRotator` 0.0 (`self.Horizontal`)) false false))
        (:`then_1`
          (`SceneComponent.K2_SetRelativeRotation` (`self.crainMain`) (`KismetMathLibrary.MakeRotator` (`self.Vertical`)) false false)
          (`SceneComponent.K2_SetRelativeLocation` (`self.crainBack`) (`KismetMathLibrary.MakeVector` 0.0 0.0 (* _langth -1.0)) false false)
          (`SceneComponent.K2_SetRelativeLocation` (`self.crainFront`) (`KismetMathLibrary.MakeVector` 0.0 0.0 (+ 84.947693 _langth)) false false)
          (`SceneComponent.K2_SetRelativeRotation` (`self.crainHandle`) (`KismetMathLibrary.MakeRotator` 0.0 0.0 (* (`self.Langth`) 30.0)) false false))
        (:`then_2`
          (`SceneComponent.K2_SetRelativeRotation` (`self.crainHead01`) (`KismetMathLibrary.MakeRotator` (* (`self.Vertical`) -1.0)) false false)
          (`SceneComponent.K2_SetRelativeRotation` (`self.crainSupportBack`) (`KismetMathLibrary.MakeRotator` (`self.Vertical`)) false false)
          (`SceneComponent.K2_SetRelativeRotation` (`self.crainSupportFront`) (`KismetMathLibrary.MakeRotator` (`self.Vertical`)) false false))
        (:`then_3`
          (`|ExecutionSequence`
            (:`then_0`
              (`SceneComponent.K2_SetRelativeLocation` _staticmesh (0.0 0.0 25.0) false false)
              (`SceneComponent.K2_SetRelativeRotation` _staticmesh (`KismetMathLibrary.MakeRotator` 0.0 (+ (- (`self.Head Rotation`) _horizontal 0.0) _horizontal)) false false))
            (:`then_1`
              (`SceneComponent.K2_SetRelativeLocation` (`self.StaticMesh1`) (`KismetMathLibrary.MakeVector` _cam_position_x (* _cam_position_y -1.0) _cam_position_z) false false)
              (`SceneComponent.K2_SetWorldTransform` (`Actor.RootComponent` (`self.Cam`)) (`KismetMathLibrary.MakeTransform` _returnvalue_location (`KismetMathLibrary.MakeRotator` 0.0 0.0 (+ (+ (`self.Head Rotation`) 90.0 0.0) (`self.Horizontal`))) (0.5 0.5 0.5)) false false))))))))

(fn `UserConstructionScript`
  (`self.Kernal`)
  (`PrimitiveComponent.SetMaterial` (`self.bodyMain`) 0 (`self.Material`))
  (`PrimitiveComponent.SetMaterial` (`self.wheel03`) 0 (`self.Material`))
  (`PrimitiveComponent.SetMaterial` (`self.wheel01`) 0 (`self.Material`))
  (`PrimitiveComponent.SetMaterial` (`self.wheel04`) 0 (`self.Material`))
  (`PrimitiveComponent.SetMaterial` (`self.crainBody`) 0 (`self.Material`))
  (`PrimitiveComponent.SetMaterial` (`self.crainSupportBack`) 0 (`self.Material`))
  (`PrimitiveComponent.SetMaterial` (`self.wheel02`) 0 (`self.Material`))
  (`PrimitiveComponent.SetMaterial` (`self.crainMain`) 0 (`self.Material`))
  (`PrimitiveComponent.SetMaterial` (`self.crainFront`) 0 (`self.Material`))
  (`PrimitiveComponent.SetMaterial` (`self.crainHead01`) 0 (`self.Material`))
  (`PrimitiveComponent.SetMaterial` (`self.crainHead02`) 0 (`self.Material`))
  (`PrimitiveComponent.SetMaterial` (`self.crainSupportFront`) 0 (`self.Material`))
  (`PrimitiveComponent.SetMaterial` (`self.crainBack`) 0 (`self.Material`))
  (`PrimitiveComponent.SetMaterial` (`self.crainHandle`) 0 (`self.Material`)))